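; Enemy AI controller that runs the BT_Enemies behavior tree and feeds perception results into its blackboard.
; On BeginPlay it starts the tree, retrying on a timer until that succeeds, then stores the pawn's location as startLocation.
; Perception updates set targetActor to the player character when sensed and clear it when lost, ignoring all other actors.
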(event `CheckBehaviourTree`
  (bind _returnvalue (`self.RunBehaviorTree` "/Game/MyContent/EnemyCharacters/AIBehaviours/BT_Enemies.BT_Enemies" :!label _label))
  (if _returnvalue
    (`self.SetDefaultKeys`)
    (else
      (`KismetSystemLibrary.K2_SetTimer` null "CheckBehaviourTree" 0.5))))

(event `self.ReceiveBeginPlay`
  (goto _label))

(event `self.AIPerception.OnTargetPerceptionUpdated`
  (params (Actor :type "Actor Object Reference") (Stimulus :type "AIStimulus Structure"))
  (bind _output_get (set `self.sensedActor` Actor))
  (if (== _output_get (`GameplayStatics.GetPlayerCharacter` 0))
    (if (`.bSuccessfullySensed` (break `AIStimulus` Stimulus))
      (`self.SetBBTargetActor` (`self.sensedActor`))
      (else
        (`self.SetBBTargetActor` null)))))

(fn `SetBBTargetActor`
  (params (actor :type "Object Object Reference"))
  (`BlackboardComponent.SetValueAsObject` (`AIBlueprintHelperLibrary.GetBlackboard` null) "targetActor" actor))

(fn `SetDefaultKeys`
  (`BlackboardComponent.SetValueAsVector` (`AIBlueprintHelperLibrary.GetBlackboard` null) "startLocation" (`self.K2_GetActorLocation` (`self.K2_GetPawn`))))

(fn `UserConstructionScript`)