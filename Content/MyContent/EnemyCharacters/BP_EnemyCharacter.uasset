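; Enemy character Blueprint that reacts to hits, shows a health bar widget and rewards the player with experience on death.
; StatsComponent's OnHit event turns the enemy toward the damage causer, launches it backward and refreshes the bar.
; Animation Blueprint messages trigger hurt or death reactions.
; On death it grants ExperienceWorth to the player's StatsComponent, hides the bar after a short delay and sets a lifespan for cleanup.
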(event `self.ReceiveBeginPlay`
  (`self.UpdateHealthPercent`))

(event `self.StatsComponent.OnHit`
  (params (isDead :type Boolean) (damageTaken :type "Float (double-precision)") (damageCauser :type "Actor Object Reference") (damageType :type "DamageType Object Reference"))
  (`self.RotateAndKnockback` damageCauser)
  (`self.UpdateHealthPercent`)
  (if isDead
    (`self.GivePlayerExperience`)
    (message `/Game/MyContent/EnemyCharacters/BI_EnemyAnimations.EAnim_Death` (`SkeletalMeshComponent.GetAnimInstance` (`self.Mesh`)))
    (`KismetSystemLibrary.Delay` 0.2)
    (`SceneComponent.SetVisibility` (`self.HealthBar`) false false)
    (`self.SetLifeSpan` 3.0)
    (else
      (message `/Game/MyContent/EnemyCharacters/BI_EnemyAnimations.EAnim_TakeDamage` (`SkeletalMeshComponent.GetAnimInstance` (`self.Mesh`))))))

(fn `GivePlayerExperience`
  (bind _asbp_agdplayer_character (cast `/Game/MyContent/PlayerCharacter/BP_AGDPlayerCharacter` (`GameplayStatics.GetPlayerCharacter` 0)))
  (`AGDStatsComponent.AddExperience` (`/Game/MyContent/PlayerCharacter/BP_AGDPlayerCharacter.StatsComponent` _asbp_agdplayer_character) (`self.experienceWorth`)))

(fn `RotateAndKnockback`
  (params (DamageCauser :type "Actor Object Reference"))
  (bind (_returnvalue_roll _returnvalue_pitch _returnvalue_yaw) (`KismetMathLibrary.BreakRotator` (`KismetMathLibrary.FindLookAtRotation` (`self.K2_GetActorLocation`) (`self.K2_GetActorLocation` DamageCauser))))
  (`self.K2_SetActorRotation` (`KismetMathLibrary.MakeRotator` 0.0 0.0 _returnvalue_yaw))
  (`self.LaunchCharacter` (* (* (`self.GetActorForwardVector`) -1.0) 750.0)))

(fn `UpdateHealthPercent`
  (bind _statscomponent (`self.StatsComponent`))
  (bind _aswui_enemy_health (cast `/Game/MyContent/EnemyCharacters/WUI_EnemyHealth` (`WidgetComponent.GetWidget` (`self.HealthBar`))))
  (`/Game/MyContent/EnemyCharacters/WUI_EnemyHealth.SetHealthPercent` _aswui_enemy_health (`AGDStatsComponent.GetHealth` _statscomponent) (`AGDStatsComponent.GetMaxHealth` _statscomponent)))

(fn `UserConstructionScript`)