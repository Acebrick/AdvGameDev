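; Player character Blueprint for a melee action game, with a StatsComponent supplying health, damage, level and experience, and a particle burst on level-up.
; Tick prints debug stats and uses controller-desired rotation only while moving with attacks allowed and no montage playing, unless rotation is forced.
; PrimaryAttack messages the AnimInstance to play a combo, while ActivateDamage and DeactivateDamage toggle a hitbox applying base damage to other actors.
; The E key grants experience directly.
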(event `self.ReceiveBeginPlay`
  (`EnhancedInputSubsystemInterface.AddMappingContext` (pcsubsystem `EnhancedInputLocalPlayerSubsystem` (`GameplayStatics.GetPlayerController` 0)) "/Game/MyContent/Input/IMC_PlayerInputMap.IMC_PlayerInputMap" 0 (struct)))

(event `self.ReceiveTick`
  (params (DeltaSeconds :type "Float (single-precision)"))
  (bind _statscomponent (`self.StatsComponent`))
  (bind (_displaylevel _displayexperience) (`AGDStatsComponent.GetDisplayLevelInfo` _statscomponent))
  (`self.HandleRotation`)
  (`KismetSystemLibrary.PrintString` (`KismetTextLibrary.Conv_TextToString` (`|FormatText` "Level: {level} \nExperience: {experience} \nHealth: {health} \nDamage: {damage}" _displaylevel _displayexperience (`AGDStatsComponent.GetHealth` _statscomponent) (`AGDStatsComponent.GetBaseDamage` _statscomponent))) true true (struct :`G` 0.66 :`B` 1.0 :`A` 1.0) 0.0))

(event `Key|E`
  (params (Key :type "Key Structure"))
  (:`Pressed`
    (`AGDStatsComponent.AddExperience` (`self.StatsComponent`) 500)))

(event `self.StatsComponent.LevelledUp`
  (params (Level :type Integer) (bAreStatsInitialised :type Boolean))
  (if bAreStatsInitialised
    (`GameplayStatics.SpawnEmitterAttached` "/Game/InfinityBladeEffects/Effects/FX_Ability/Heal/P_Health_Pickup_01.P_Health_Pickup_01" (`self.Mesh`))))

(event `self.DamageHitBox.OnComponentBeginOverlap`
  (params (OverlappedComponent :type "PrimitiveComponent Object Reference") (OtherActor :type "Actor Object Reference") (OtherComp :type "PrimitiveComponent Object Reference") (OtherBodyIndex :type Integer) (bFromSweep :type Boolean) (SweepResult :type "HitResult Structure (by ref)"))
  ;[1 1 1] Apply damage to everything but self
  (if (!= OtherActor self)
    (`GameplayStatics.ApplyDamage` OtherActor (`KismetMathLibrary.Conv_IntToDouble` (`AGDStatsComponent.GetBaseDamage` (`self.StatsComponent`))) null self)))

(fn `ActivateDamage`
  (`PrimitiveComponent.SetCollisionEnabled` (`self.DamageHitBox`) "QueryOnly"))

(fn `DeactivateDamage`
  (`PrimitiveComponent.SetCollisionEnabled` (`self.DamageHitBox`) "NoCollision"))

(fn `HandleRotation`
  (set `CharacterMovementComponent.bUseControllerDesiredRotation` (or (and (> (`KismetMathLibrary.VSizeXY` (`self.GetVelocity`)) 0.0) (`self.GetAttackAllowed`) (not (`self.IsAnyMontagePlaying`))) (`self.GetForceRotate`)) (`self.CharacterMovement`)))

(fn `IsAnyMontagePlaying`
  (returns (bIsAnyMontagePlaying :type Boolean))
  (return (`AnimInstance.IsAnyMontagePlaying` (`SkeletalMeshComponent.GetAnimInstance` (`self.Mesh`)))))

(fn `PrimaryAttack`
  (message `/Game/MyContent/PlayerCharacter/BI_PlayerAnimations.PlayComboAttack` (`SkeletalMeshComponent.GetAnimInstance` (`self.Mesh`)) 1.0))

(fn `UserConstructionScript`)