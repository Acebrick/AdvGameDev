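; BP_StatsComponent is an actor component that tracks its owner's health and death state.
; On BeginPlay it binds to the owner's take-any-damage event and ignores further hits once dead.
; HandleDamage subtracts damage from health clamped between zero and max, sets IsDead at zero, then broadcasts OnHit with the death flag and damage details.
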(event `self.ReceiveBeginPlay`
  (add `Actor.OnTakeAnyDamage` (`self.GetOwner`) (delegate `OnOwnerTakeAnyDamage`)))

(event `OnOwnerTakeAnyDamage`
  (params (DamagedActor :type "Actor Object Reference") (Damage :type "Float (single-precision)") (DamageType :type "DamageType Object Reference") (InstigatedBy :type "Controller Object Reference") (DamageCauser :type "Actor Object Reference"))
  (if (not (`self.GetIsDead`))
    (`self.HandleDamage` Damage DamageCauser DamageType)))

(fn `GetIsDead`
  (returns (isDead :type Boolean))
  (return (`self.isDead`)))

(fn `HandleDamage`
  (params (damageTaken :type "Float (double-precision)") (damageCauser :type "Actor Object Reference") (damageType :type "DamageType Object Reference"))
  (locals (lDamageTaken :type "Float (double-precision)") (lDamageCauser :type "Actor Object Reference") (lDamageType :type "DamageType Object Reference"))
  (set `local.lDamageCauser` damageCauser)
  (set `local.lDamageType` damageType)
  (set `local.lDamageTaken` damageTaken)
  (`self.SetHealth` (`KismetMathLibrary.FClamp` (- (`self.GetHealth`) damageTaken) 0.0 (`self.GetMaxHealth`)))
  (bind _output_get (set `self.isDead` (<= (`self.GetHealth`) 0.0)))
  (`self.OnHit` _output_get (`local.lDamageTaken`) (`local.lDamageCauser`) (`local.lDamageType`)))